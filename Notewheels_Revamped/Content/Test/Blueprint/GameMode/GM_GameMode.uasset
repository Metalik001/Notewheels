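; Game mode for a rhythm game that starts the music Level Sequence, exposes its playback time and the global note travel time, and tracks score and combo.
; Combo changes update the HUD and raise the score multiplier every ten notes.
; Button presses go to the lowest-indexed BPI_ButtonNote actor.
; Long-note touches within an index tolerance award points with throttled sound and destroy the note, plus skipped segments.
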(event EventResetCombo
  ;[1 1 1] Reset Combo
  (bind _output_get (Variables|Default|SetCombo 0))
  (Class|BPIHUD|SetCombo(Message) (HUD|GetHUD (Game|GetPlayerController 0)) _output_get))

(event EventTouchedLongNote
  (params (IndexActual :type Integer) (NoteToDelete :type Actor%20Object%20Reference))
  (bind _notesspawned (Variables|Default|GetNotesSpawned))
  ;[1 1 1] Tolerance
  (Utilities|Array|Add (Variables|Default|GetNotesSpawned) NoteToDelete)
  (if (Math|Integer|InRange(Integer) IndexActual (Variables|Default|GetPreviousIndex) (+ (Variables|Default|GetPreviousIndex) 5))
    ;[1 1 1] Allow the long note to be counted
    (Utilities|FlowControl|Sequence
      (:then_0
        ;[1 1 1] Play sound
        (Utilities|FlowControl|DoOnce false :!label _label
          (:Completed
            (Audio|PlaySound2D "/Game/Test/Sound_Effects/SC_GoodNote_Cue.SC_GoodNote_Cue" 1.0 1.0 0.0 0 0)
            (Utilities|FlowControl|Delay 0.1)
            (goto _label Reset))))
      (:then_1
        (Class|BPIGameMode|AddScore(Message) self 10)
        (Actor|DestroyActor NoteToDelete)
        (Utilities|FlowControl|RetriggerableDelay 0.2)
        (Variables|Default|SetPreviousIndex 0)
        (Utilities|Array|Clear (Variables|Default|GetNotesSpawned)))
      (:then_2
        ;[1 1 1] Supprime les éléments mis avants si pas touchés
        (if (not (Math|Integer|InRange(Integer) IndexActual (- (Variables|Default|GetPreviousIndex) 10) (Variables|Default|GetPreviousIndex)))
          (for _index (range (Variables|Default|GetPreviousIndex) IndexActual)
            (if (Utilities|Array|IsValidIndex _notesspawned _index)
              (Utilities|IsValid (Utilities|Array|Get(acopy) _notesspawned _index)
                (:Is%20Valid
                  (Actor|DestroyActor (Utilities|Array|Get(acopy) _notesspawned _index)))))))
        (Variables|Default|SetPreviousIndex IndexActual)))))

(event EventSetGlobalTravelTime
  (params (NewValue :type Float%20%28double-precision%29))
  ;[1 1 1] Set new Global Travel Time
  (Variables|Default|SetGlobalTravelTime NewValue))

(event EventAddNotetoCombo
  ;[1 1 1] Add Note to the combo
  (bind _result (Math|Integer|IncrementInt (Variables|Default|GetCombo))
    (:%20%20
      (bind _output_get (Variables|Default|SetCombo _result))
      (Class|BPIHUD|SetCombo(Message) (HUD|GetHUD (Game|GetPlayerController 0)) _output_get))))

(event EventAddScore
  (params (ScoreToAdd :type Integer))
  ;[1 1 1] Add the score of the note to the overall score
  (bind _output_get (Variables|Default|SetScore (+ (* ScoreToAdd (+ (/ (Variables|Default|GetCombo) 10) 1)) (Variables|Default|GetScore))))
  (Class|BPIHUD|SetScore(Message) (HUD|GetHUD (Game|GetPlayerController 0)) _output_get))

(event EventButtonPressed
  (bind _buttonindexes (Variables|Default|GetButtonIndexes))
  ;[1 1 1] Vérification des notes
  (bind _outactors (Actor|GetAllActorswithInterface "/Game/Test/Blueprint/Interface/BPI_ButtonNote.BPI_ButtonNote_C"))
  (for _array_element _outactors
    (bind _index (Class|BPIButtonNote|GetIndex(Message) _array_element))
    (Utilities|Array|Add _buttonindexes _index))
  (Class|BPIButtonNote|ButtonPressed(Message) (Utilities|Array|Get(acopy) _outactors (.IndexOfMinValue (Math|Integer|MinOfIntArray (Variables|Default|GetButtonIndexes)))))
  (Utilities|Array|Clear _buttonindexes))

(event EventBeginPlay
  ;[1 0 0] BeginPlay
  (Utilities|Array|Clear (Variables|Default|GetNotesSpawned))
  (bind _returnvalue (Sequencer|Player|CreateLevelSequencePlayer "/Game/Test/Level_Sequences/Test.Test"))
  (bind _output_get (Variables|Default|SetMusic%20played _returnvalue))
  (Utilities|FlowControl|Delay 0.2)
  (Sequencer|Player|Play _output_get :!class /Script/MovieScene.MovieSceneSequencePlayer))

(fn ConstructionScript)

(fn GetCurrentMusicTime
  ;[1 1 1] Récupère la frame exacte à l'instant.
  (return (Sequencer|Player|GetCurrentTime (Variables|Default|GetMusic%20played))))

(fn GetGlobalTravelTime
  ;[1 1 1] Global Travel Time
  (return (Variables|Default|GetGlobalTravelTime)))
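; BP_Note is a rhythm-game note actor that scores when its Background component is overlapped and counts as a miss otherwise.
; A miss after TimeToReachTheEnd plays a bad sound, resets the combo and destroys it.
; An overlap line-traces toward Sphere, doubles points on "Great"-tagged hits, then messages the GameMode for score and combo.
; The construction script yaws Background toward Destination; movement and spin timelines are unconnected.
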(event OnComponentBeginOverlap(Background)
  (params (OverlappedComponent :type Primitive%20Component%20Object%20Reference) (OtherActor :type Actor%20Object%20Reference) (OtherComp :type Primitive%20Component%20Object%20Reference) (OtherBodyIndex :type Integer) (bFromSweep :type Boolean) (SweepResult :type Hit%20Result%20Structure%20%28by%20ref%29))
  ;[1 1 1] Special check
  (bind _outhit (Collision|LineTraceByChannel (Transformation|GetWorldLocation (Variables|Default|GetBackground)) (Transformation|GetWorldLocation (Variables|Default|GetSphere)) "TraceTypeQuery1" false 0 "None"))
  (Utilities|IsValid (.HitComponent (Collision|BreakHitResult _outhit))
    (:Is%20Valid
      (if (Utilities|Array|ContainsItem (Variables|/Script/Engine.ActorComponent|GetComponentTags (.HitComponent (Collision|BreakHitResult _outhit))) "Great")
        ;[1 1 1] Stops the mouvement and make it disapear if the player touches it
        (Variables|Default|SetPointsToScore (* (Variables|Default|GetPointsToScore) 2))))
    (:Is%20Not%20Valid
      _))
  (Class|BPIGameMode|AddScore(Message) (Game|GetGameMode) (Variables|Default|GetPointsToScore))
  (Audio|PlaySound2D "/Game/Test/Sound_Effects/SC_GoodNote_Cue.SC_GoodNote_Cue" 1.0 1.0 0.0 0 0)
  (Class|BPIGameMode|AddNotetoCombo(Message) (Game|GetGameMode))
  (Actor|DestroyActor))

(event EventBeginPlay
  ;[1 1 1] When it's arrived, gets deleted
  (Utilities|FlowControl|Delay (Variables|Default|GetTime%20to%20reach%20the%20end))
  (Audio|PlaySound2D "/Game/Test/Sound_Effects/SC_BadNote_Cue.SC_BadNote_Cue" 1.0 1.0 0.0 0 0)
  (Class|BPIGameMode|ResetCombo(Message) (Game|GetGameMode))
  (Actor|DestroyActor))

(fn ConstructionScript
  (bind _background (Variables|Default|GetBackground))
  ;[1 1 1] Changes the rotation of the background
  (Transformation|SetRelativeRotation _background (Math|Rotator|MakeRotator 9e+01 0.0 (.Yaw (Math|Rotator|BreakRotator (Math|Rotator|FindLookatRotation (Transformation|GetWorldLocation _background) (Variables|Default|GetDestination))))) false false))
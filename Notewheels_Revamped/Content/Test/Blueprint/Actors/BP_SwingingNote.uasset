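; BP_SwingingNote is a rhythm-game note that, once touched, must be swung back and forth between two points a set number of times.
; On first overlap it attaches to the touching component and reveals a target that alternates sides per hit, awarding score.
; A timeline drains a radial confirm bar; missing the note or running out resets combo, while the last hit gives bonus score.
; The construction script builds dynamic materials for the bar and directional arrow arc.
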(event OnComponentBeginOverlap(MainNoteBackground)
  (params (OverlappedComponent :type Primitive%20Component%20Object%20Reference) (OtherActor :type Actor%20Object%20Reference) (OtherComp :type Primitive%20Component%20Object%20Reference) (OtherBodyIndex :type Integer) (bFromSweep :type Boolean) (SweepResult :type Hit%20Result%20Structure%20%28by%20ref%29))
  ;[1 1 1] Starts swing mode
  (Utilities|FlowControl|DoOnce false
    (:Completed
      (Transformation|AttachComponentToComponent (Variables|Default|GetMain%20Note%20Background) OtherComp "None" "SnapToTarget" "KeepWorld" "KeepWorld" true)
      (Audio|PlaySound2D "/Game/Test/Sound_Effects/SC_GoodNote_Cue.SC_GoodNote_Cue" 1.0 1.0 0.0 0 0)
      (CallFunction|Swinging))))

(event OnComponentBeginOverlap(Background1)
  (params (OverlappedComponent :type Primitive%20Component%20Object%20Reference) (OtherActor :type Actor%20Object%20Reference) (OtherComp :type Primitive%20Component%20Object%20Reference) (OtherBodyIndex :type Integer) (bFromSweep :type Boolean) (SweepResult :type Hit%20Result%20Structure%20%28by%20ref%29))
  ;[1 1 1] Touching Background
  (if (and (== OtherComp (Variables|Default|GetMain%20Note%20Background)) (Variables|Default|GetTouched))
    (if (> (Variables|Default|GetTimesToHit) 1)
      (CallFunction|SwingingHit)
      (else
        (CallFunction|GoodNote)))))

(event Custom|StopMovement
  (bind _time_to_reach_the_end (Variables|Default|GetTime%20to%20reach%20the%20end))
  ;[1 1 1] Movement
  (bind _mouvement (Timeline|Movement Stop)
    (:Update
      ;[1 1 1] Goes to targetted destination
      (Transformation|SetRelativeLocation (Variables|Default|GetMain%20Note%20Background) (+ (Math|Vector|Lerp(Vector) "0, 0, 0" (Variables|Default|GetDestination) (/ _mouvement _time_to_reach_the_end)) "0.000000,0.000000,5.000000") false false)
      (Utilities|FlowControl|DoOnce false
        (:Completed
          (Transformation|SetRelativeLocation (Variables|Default|GetBackground1) (+ (Variables|Default|GetSwingDestination) "0.000000,0.000000,5.000000") false false))))))

(event Custom|Swinging
  (bind _main_note_background (Variables|Default|GetMain%20Note%20Background))
  ;[1 1 1] Sets the note to the swinging state
  (Collision|SetCollisionObjectType _main_note_background "ECC_WorldStatic")
  (Collision|SetCollisionResponsetoChannel _main_note_background "ECC_WorldStatic" "ECR_Overlap")
  (Development|SetHiddeninGame (Variables|Default|GetBackground1) false true)
  (Variables|Default|SetTouched true)
  (CallFunction|StopMovement)
  (CallFunction|SetTimeLeft)
  (Rendering|Components|TextRender|SetText (Variables|Default|GetTextRender) (Utilities|Text|ToText(Integer) (Variables|Default|GetTimesToHit))))

(event Custom|GoodNote
  ;[1 1 1] La note est comptée
  (Audio|PlaySound2D "/Game/Test/Sound_Effects/SC_GoodNote_Cue.SC_GoodNote_Cue" 1.0 1.0 0.0 0 0)
  (Class|BPIGameMode|AddScore(Message) (Game|GetGameMode) (* (Variables|Default|GetPointsToScore) 5))
  (Actor|DestroyActor))

(event Custom|BadNote
  ;[1 1 1] Failed
  (Audio|PlaySound2D "/Game/Test/Sound_Effects/SC_BadNote_Cue.SC_BadNote_Cue" 1.0 1.0 0.0 0 0)
  (Class|BPIGameMode|ResetCombo(Message) (Game|GetGameMode))
  (Actor|DestroyActor))

(event Custom|SwingingHit
  (bind _background1 (Variables|Default|GetBackground1))
  (bind _arrowcirclematerial (Variables|Default|GetArrowCircleMaterial))
  ;[1 1 1] Lorsque la note se retrouve au point
  (bind _result (Math|Integer|DecrementInt (Variables|Default|GetTimesToHit))
    (:%20%20
      (Rendering|Components|TextRender|SetText (Variables|Default|GetTextRender) (Utilities|Text|ToText(Integer) _result))
      (Utilities|FlowControl|FlipFlop
        (:A
          (Transformation|SetRelativeLocation _background1 (+ (* (Variables|Default|GetDestination) 0.8) "0.000000,0.000000,5.000000") false false))
        (:B
          (Transformation|SetRelativeLocation _background1 (+ (Variables|Default|GetSwingDestination) "0.000000,0.000000,5.000000") false false)))
      (Audio|PlaySound2D "/Game/Test/Sound_Effects/SC_GoodNote_Cue.SC_GoodNote_Cue" 1.0 1.0 0.0 0 0)
      (Class|BPIGameMode|AddScore(Message) (Game|GetGameMode) (Variables|Default|GetPointsToScore))
      (bind _returnvalue (Rendering|Material|GetScalarParameterValue _arrowcirclematerial "Direction" :!class /Script/Engine.MaterialInstanceDynamic))
      (Rendering|Material|SetScalarParameterValue _arrowcirclematerial "Direction" (* _returnvalue -1.0) :!class /Script/Engine.MaterialInstanceDynamic))))

(event Custom|SetTimeLeft
  (bind _timetoconfirm (Variables|Default|GetTimeToConfirm))
  ;[1 1 1] Radial Bar decrease
  (bind _mouvement (Timeline|Timeline Play)
    (:Update
      (Rendering|Material|SetScalarParameterValue (Variables|Default|GetCircularBarMat) "Percent" (Math|Float|Lerp 1.0 0.0 (/ _mouvement _timetoconfirm)) :!class /Script/Engine.MaterialInstanceDynamic)
      (if (>= (/ _mouvement _timetoconfirm) 1.0)
        (CallFunction|BadNote)))))

(event EventBeginPlay
  ;[1 0 0] When it's arrived, gets deleted
  (Utilities|FlowControl|Delay (Variables|Default|GetTime%20To%20Reach%20The%20End))
  (if (not (Variables|Default|GetTouched))
    (CallFunction|BadNote)))

(fn ConstructionScript
  (bind _cercle1 (Variables|Default|GetCercle1))
  ;[1 1 1] Création du matérial radial bar
  (bind _returnvalue (Rendering|Material|CreateDynamicMaterialInstance (Variables|Default|GetBackground1) 0 "/Game/Test/Material/M_RadialBar.M_RadialBar" "None" :!class /Script/Engine.PrimitiveComponent))
  (bind _output_get (Variables|Default|SetCircularBarMat _returnvalue))
  (Rendering|Material|SetVectorParameterValue _output_get "Color" "(R=0.075101,G=1.000000,B=0.000000,A=1.000000)" :!class /Script/Engine.MaterialInstanceDynamic)
  ;[1 1 1] Cration de l'arrows ring
  (bind _returnvalue_2 (Rendering|Material|CreateDynamicMaterialInstance (Variables|Default|GetCercle1) 0 "/Game/Test/Material/M_TestNewSprite.M_TestNewSprite" "None" :!class /Script/Engine.PrimitiveComponent))
  (Variables|Default|SetArrowCircleMaterial _returnvalue_2)
  (Utilities|TurnIntoPositiveAngle
    (:Positive
      (if (Variables|Default|GetFlip)
        (Transformation|SetRelativeRotation _cercle1 (Math|Rotator|MakeRotator -9e+01 0.0 (+ 9e+01 (* -1.0 (Variables|Default|GetSwingDestinationAngle)))) false false)
        (Rendering|Material|SetScalarParameterValue (Variables|Default|GetArrowCircleMaterial) "Direction" 1.0 :!class /Script/Engine.MaterialInstanceDynamic)
        (else
          (Transformation|SetRelativeRotation _cercle1 (Math|Rotator|MakeRotator -9e+01 0.0 (+ 9e+01 (* (Variables|Default|GetDestinationAngle) -1.0))) false false)
          (Rendering|Material|SetScalarParameterValue (Variables|Default|GetArrowCircleMaterial) "Direction" -1.0 :!class /Script/Engine.MaterialInstanceDynamic)))
      (CallFunction|CalculatePercentage))))

(fn CalculatePercentage
  ;[1 1 1] calculates the percentage for the swing ring
  (bind _result (Utilities|TurnIntoPositiveAngle)
    (:Positive
      (if (Variables|Default|GetFlip)
        (LocalVariables|SetPercentage (- 1.0 (/ _result 3.6e+02)))
        (else
          (LocalVariables|SetPercentage (/ _result 3.6e+02))))
      (Rendering|Material|SetScalarParameterValue (Variables|Default|GetArrowCircleMaterial) "Percent" (LocalVariables|GetPercentage) :!class /Script/Engine.MaterialInstanceDynamic))))
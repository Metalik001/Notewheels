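; Rhythm-style note actor that travels to a destination, bounces on its first overlap and counts as a hit on the second.
; The Movement timeline drives a straight lerp, then a quadratic Bézier bounce through the spawn point, with collision briefly disabled and the indicator shown.
; Both overlaps award points, the second adding combo and destroying the note.
; A retriggerable delay destroys expired notes as misses, resetting the combo.
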(event OnComponentBeginOverlap(Background)
  (params (OverlappedComponent :type Primitive%20Component%20Object%20Reference) (OtherActor :type Actor%20Object%20Reference) (OtherComp :type Primitive%20Component%20Object%20Reference) (OtherBodyIndex :type Integer) (bFromSweep :type Boolean) (SweepResult :type Hit%20Result%20Structure%20%28by%20ref%29))
  (bind _returnvalue (Game|GetGameMode))
  (bind _defaultsceneroot (Variables|Default|GetDefaultSceneRoot))
  (bind _relativelocation (Variables|/Script/Engine.SceneComponent|GetRelativeLocation _defaultsceneroot))
  (bind (_x _y) (Math|Vector|BreakVector _relativelocation))
  ;[1 1 1] La fait sauter une fois puis disparaitre une seconde fois
  (Utilities|FlowControl|FlipFlop
    (:A
      (Variables|Default|SetStartLocation (Math|Vector|MakeVector _x _y 5.0))
      (Rendering|SetActorHiddenInGame (Variables|Default|GetBP_Indicator) false)
      (Variables|Default|SetBouncing true)
      (CallFunction|Prevention)
      (Class|BPIGameMode|AddScore(Message) (Game|GetGameMode) (Variables|Default|GetPointsToScore))
      (CallFunction|BounceTravel))
    (:B
      ;[1 1 1] La note est comptée
      (Audio|PlaySound2D "/Game/Test/Sound_Effects/SC_GoodNote_Cue.SC_GoodNote_Cue" 1.0 1.0 0.0 0 0)
      (Class|BPIGameMode|AddScore(Message) _returnvalue (* (Variables|Default|GetPointsToScore) 3))
      (Class|BPIGameMode|AddNotetoCombo(Message) _returnvalue)
      (Actor|DestroyActor self))))

(event Custom|Prevention
  (bind _background (Variables|Default|GetBackground))
  ;[1 1 1] Prevents that the notes gets counted at the start
  (Collision|SetCollisionEnabled _background "NoCollision")
  (Utilities|FlowControl|Delay (/ (Variables|Default|GetBounceTime) 2.0))
  (Collision|SetCollisionEnabled _background "QueryAndPhysics"))

(event Custom|BounceTravel
  (bind _time_to_reach_the_end (Variables|Default|GetTime%20to%20reach%20the%20end))
  ;[1 1 1] Movement
  (Variables|Default|SetTime%20To%20Reach%20The%20End (Variables|Default|GetBounceTime))
  (CallFunction|RetriggerTimer)
  (bind _mouvement (Timeline|Movement PlayFromStart)
    (:Update
      (if (Variables|Default|GetBouncing)
        ;[1 1 1] Bounce movement
        (bind _beziercurve (CallFunction|GotBounced (Variables|Default|GetStartLocation) (Variables|Default|GetSpawnLocation) (+ (Variables|Default|GetBounceDestination) "0.000000,0.000000,5.000000") (/ _mouvement _time_to_reach_the_end)))
        (Transformation|SetRelativeLocation (Variables|Default|GetDefaultSceneRoot) _beziercurve false false)
        (else
          ;[1 1 1] Goes to targetted destination
          (Transformation|SetRelativeLocation (Variables|Default|GetDefaultSceneRoot) (+ (Math|Vector|Lerp(Vector) "0, 0, 0" (Variables|Default|GetDestination) (/ _mouvement _time_to_reach_the_end)) "0.000000,0.000000,5.000000") false false))))))

(event Custom|Retrigger%20Timer
  (bind _bp_indicator (Variables|Default|GetBP_Indicator))
  ;[1 0 0] When it's arrived, gets deleted
  (Utilities|FlowControl|RetriggerableDelay (Variables|Default|GetTime%20To%20Reach%20The%20End))
  (Audio|PlaySound2D "/Game/Test/Sound_Effects/SC_BadNote_Cue.SC_BadNote_Cue" 1.0 1.0 0.0 0 0)
  (Class|BPIGameMode|ResetCombo(Message) (Game|GetGameMode))
  (Utilities|FlowControl|Sequence
    (:then_0
      (Actor|DestroyActor))
    (:then_1
      (Utilities|IsValid _bp_indicator
        (:Is%20Valid
          (Actor|DestroyActor _bp_indicator))))))

(event EventBeginPlay
  (bind _returnvalue (Transformation|GetActorLocation))
  (bind _bp_indicator (Variables|Default|GetBP_Indicator))
  (bind (_x _y) (Math|Vector|BreakVector _returnvalue))
  ;[1 0 0] When it's arrived, gets deleted
  (Variables|Default|SetSpawnLocation (Math|Vector|MakeVector _x _y 5.0))
  (Utilities|FlowControl|RetriggerableDelay (Variables|Default|GetTime%20To%20Reach%20The%20End))
  (Audio|PlaySound2D "/Game/Test/Sound_Effects/SC_BadNote_Cue.SC_BadNote_Cue" 1.0 1.0 0.0 0 0)
  (Class|BPIGameMode|ResetCombo(Message) (Game|GetGameMode))
  (Utilities|FlowControl|Sequence
    (:then_0
      (Actor|DestroyActor))
    (:then_1
      (Utilities|IsValid _bp_indicator
        (:Is%20Valid
          (Actor|DestroyActor _bp_indicator))))))

(fn ConstructionScript)

(fn GotBounced
  (params (Start :type Vector) (Middle :type Vector) (End :type Vector) (Time :type Float%20%28double-precision%29))
  (Utilities|FlowControl|Sequence
    (:then_0
      (LocalVariables|SetMiddle_A (Math|Vector|Lerp(Vector) Start Middle Time))
      (LocalVariables|SetMiddle_B (Math|Vector|Lerp(Vector) Middle End Time)))
    (:then_1
      (return (Math|Vector|Lerp(Vector) (LocalVariables|GetMiddle_A) (LocalVariables|GetMiddle_B) Time)))))
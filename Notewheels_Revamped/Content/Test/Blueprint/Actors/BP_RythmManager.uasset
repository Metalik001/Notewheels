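; Rhythm game manager that exposes events to spawn each note type at the player: single, circular, big, bouncing, long, mashing and swinging.
; Directional notes rotate the player's SpawnerNotes component to derive a fixed-radius destination, then every note is attached to P_Player.
; Circular, big and mashing notes share an index and register with the game mode.
; Long notes sweep direction on a Timeline, spawning segments per update, with a retriggerable delay resetting their index.
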(event Custom|SpawnSingleNote
  (params (Direction :type Float%20%28double-precision%29) (TravelTime :type Float%20%28double-precision%29))
  ;[1 1 1] Spawn Single Note
  (CallFunction|ChangeDirection Direction)
  (bind _returnvalue (Game|SpawnActorfromClass "/Game/Test/Blueprint/Actors/BP_Note.BP_Note_C" (Math|Transform|MakeTransform (Transformation|GetActorLocation (Game|Player|GetPlayerPawn 0))) "Undefined" "MultiplyWithRoot" 0 (Variables|Default|GetEnd%20point) TravelTime 0))
  (CallFunction|AttachtoPlayer _returnvalue))

(event Custom|Spawn_SwingingNote
  (params (Direction :type Float%20%28double-precision%29) (Swing%20Direction :type Float%20%28double-precision%29) (Time%20To%20Reach%20The%20End :type Float%20%28double-precision%29) (TimeToConfirm :type Float%20%28double-precision%29) (TimesToHit :type Integer) (Flip :type Boolean))
  ;[1 1 1] Spawn Swinging Note
  (CallFunction|ChangeDirection Swing%20Direction)
  (Variables|Default|SetSwingPos (* (Variables|Default|GetEnd%20point) 0.8))
  (CallFunction|ChangeDirection Direction)
  (bind _returnvalue (Game|SpawnActorfromClass "/Game/Test/Blueprint/Actors/BP_SwingingNote.BP_SwingingNote_C" (Math|Transform|MakeTransform (Transformation|GetActorLocation (Game|Player|GetPlayerPawn 0))) "Undefined" "MultiplyWithRoot" 0 (Variables|Default|GetEnd%20point) Time%20To%20Reach%20The%20End TimeToConfirm (Variables|Default|GetSwingPos) TimesToHit Direction Swing%20Direction Flip 0))
  (CallFunction|AttachtoPlayer _returnvalue))

(event Custom|SpawnCircularNote
  (params (Time%20To%20Reach%20The%20End :type Float%20%28double-precision%29))
  ;[1 1 1] Spawn Circular note
  (bind _returnvalue (Game|SpawnActorfromClass "/Game/Test/Blueprint/Actors/BP_CircularNote.BP_CircularNote_C" (Math|Transform|MakeTransform (+ (Transformation|GetActorLocation (Game|Player|GetPlayerPawn 0)) "0.000000,0.000000,20.000000")) "Undefined" "MultiplyWithRoot" 0 (Variables|Default|GetIndexOfButtonNote) Time%20To%20Reach%20The%20End 0))
  (CallFunction|AttachtoPlayer _returnvalue)
  (Class|BPIGameMode|AddButtonNote(Message) (Game|GetGameMode) _returnvalue)
  (Variables|Default|SetIndexOfButtonNote (+ (Variables|Default|GetIndexOfButtonNote) 1)))

(event Custom|Anim
  ;[1 1 1] Flip animation
  (Default|FlipAnim (Variables|Default|GetP_Player)))

(event Custom|SpawnBigNote
  (params (Direction :type Float%20%28double-precision%29) (TravelTime :type Float%20%28double-precision%29))
  ;[1 1 1] Spawns BigNote
  (CallFunction|ChangeDirection Direction)
  (bind _returnvalue (Game|SpawnActorfromClass "/Game/Test/Blueprint/Actors/BP_BigNote.BP_BigNote_C" (Math|Transform|MakeTransform (Transformation|GetActorLocation (Game|Player|GetPlayerPawn 0))) "Undefined" "MultiplyWithRoot" 0 (Variables|Default|GetEnd%20point) TravelTime (Variables|Default|GetIndexOfButtonNote) 0))
  (CallFunction|AttachtoPlayer _returnvalue)
  (Class|BPIGameMode|AddButtonNote(Message) (Game|GetGameMode) _returnvalue)
  (Variables|Default|SetIndexOfButtonNote (+ (Variables|Default|GetIndexOfButtonNote) 1)))

(event Custom|SpawnBouncingNote
  (params (Direction :type Float%20%28double-precision%29) (BounceDirection :type Float%20%28double-precision%29) (TravelTime :type Float%20%28double-precision%29) (BounceTime :type Float%20%28double-precision%29))
  (bind _returnvalue (Game|Player|GetPlayerPawn 0))
  (bind _returnvalue_2 (Transformation|GetActorLocation _returnvalue))
  (bind _returnvalue_3 (Math|Transform|MakeTransform _returnvalue_2))
  ;[1 1 1] Spawn Bouncing Note
  (CallFunction|ChangeDirection BounceDirection)
  (bind _output_get (Variables|Default|SetBouncePos (Variables|Default|GetEnd%20point)))
  (bind _returnvalue_4 (Game|SpawnActorfromClass "/Game/Test/Blueprint/Actors/BP_IndicatorBouncingNote.BP_IndicatorBouncingNote_C" _returnvalue_3 "Undefined" "MultiplyWithRoot" 0 (* _output_get 0.8) 0))
  (CallFunction|AttachtoPlayer _returnvalue_4)
  (CallFunction|ChangeDirection Direction)
  (bind _returnvalue_5 (Game|SpawnActorfromClass "/Game/Test/Blueprint/Actors/BP_BouncingNote.BP_BouncingNote_C" _returnvalue_3 "Undefined" "MultiplyWithRoot" 0 (Variables|Default|GetEnd%20point) _returnvalue_4 TravelTime BounceTime (Variables|Default|GetBouncePos) 0))
  (CallFunction|AttachtoPlayer _returnvalue_5))

(event Custom|Change%20Direction
  (params (New%20direction :type Float%20%28double-precision%29))
  ;[1 1 1] Change la direction pour les notes
  (Transformation|SetRelativeRotation (Variables|/Game/Test/Blueprint/Pawn/P_Player.P_Player_C|GetSpawner%20notes (Variables|Default|GetP_Player)) (Math|Rotator|MakeRotator 0.0 New%20direction 0.0) false false)
  (CallFunction|SetDestination))

(event Custom|Attach%20to%20Player
  (params (Target :type Actor%20Object%20Reference))
  ;[1 1 1] Attache au joueur
  (Transformation|AttachActorToActor Target (Variables|Default|GetP_Player) "None" "KeepWorld" "KeepRelative" "KeepWorld" false))

(event Custom|Set%20Destination
  (bind _p_player (Variables|Default|GetP_Player))
  (bind _spawner_notes (Variables|/Game/Test/Blueprint/Pawn/P_Player.P_Player_C|GetSpawner%20notes _p_player))
  (bind _returnvalue (Math|Vector|GetForwardVector _spawner_notes))
  (bind (_x _y) (Math|Vector|BreakVector _returnvalue))
  ;[1 1 1] Destination
  (Variables|Default|SetEnd%20point (* (Math|Vector|MakeVector _x _y 0.0) 280)))

(event Custom|SpawnLongNote
  (params (Direction :type Float%20%28double-precision%29) (TravelTime :type Float%20%28double-precision%29) (TimeToOtherDirection :type Float%20%28single-precision%29) (NewDirection :type Float%20%28double-precision%29))
  ;[1 1 1] Goes from one point to another
  (Utilities|FlowControl|Sequence
    (:then_0
      (bind _mouvement (Timeline|Timeline_0 PlayFromStart)
        (:Update
          (CallFunction|ChangeDirection (Math|Float|Lerp Direction NewDirection (/ _mouvement TimeToOtherDirection)))
          (if (== (Variables|Default|GetIndexOfSegment) 0)
            ;[1 1 1] Start of the segment
            (bind _returnvalue (Game|SpawnActorfromClass "/Game/Test/Blueprint/Actors/BP_LongNoteStart.BP_LongNoteStart_C" (Math|Transform|MakeTransform (Transformation|GetActorLocation (Game|Player|GetPlayerPawn 0))) "Undefined" "MultiplyWithRoot" 0 (Variables|Default|GetEnd%20point) TravelTime (Variables|Default|GetIndexOfSegment) 0))
            (CallFunction|AttachtoPlayer _returnvalue)
            (else
              ;[1 1 1] Spawn Long Note Segement
              (bind _returnvalue_2 (Game|SpawnActorfromClass "/Game/Test/Blueprint/Actors/BP_LongNoteSegments.BP_LongNoteSegments_C" (Math|Transform|MakeTransform (Transformation|GetActorLocation (Game|Player|GetPlayerPawn 0))) "Undefined" "MultiplyWithRoot" 0 (Variables|Default|GetEnd%20point) (Variables|Default|GetIndexOfSegment) TravelTime 0))
              (CallFunction|AttachtoPlayer _returnvalue_2)))
          ;[1 1 1] Index resets when it ends to spawn
          (Variables|Default|SetIndexOfSegment (+ (Variables|Default|GetIndexOfSegment) 1))
          (Utilities|FlowControl|RetriggerableDelay 0.2)
          (Variables|Default|SetIndexOfSegment 0))))
    (:then_1
      (Utilities|FlowControl|Delay TimeToOtherDirection)
      (Timeline|Timeline_0 Stop))))

(event Custom|ChangeGlobalTravelTime
  (params (NewTravelTime :type Float%20%28double-precision%29))
  ;[1 1 1] Set Global travel time
  (Class|BPIGameMode|SetGlobalTravelTime(Message) (Game|GetGameMode) NewTravelTime))

(event Custom|Spawn_MashNote
  (params (Time%20To%20Reach%20The%20End :type Float%20%28double-precision%29) (TimesToMash :type Integer) (Time%20To%20ConfirmNote :type Float%20%28double-precision%29))
  ;[1 1 1] Spawn Mashing note
  (bind _returnvalue (Game|SpawnActorfromClass "/Game/Test/Blueprint/Actors/BP_CircularNoteTapping.BP_CircularNoteTapping_C" (Math|Transform|MakeTransform (+ (Transformation|GetActorLocation (Game|Player|GetPlayerPawn 0)) "0.000000,0.000000,20.000000")) "Undefined" "MultiplyWithRoot" 0 (Variables|Default|GetIndexOfButtonNote) Time%20To%20Reach%20The%20End TimesToMash Time%20To%20ConfirmNote 0))
  (CallFunction|AttachtoPlayer _returnvalue)
  (Class|BPIGameMode|AddButtonNote(Message) (Game|GetGameMode) _returnvalue)
  (Variables|Default|SetIndexOfButtonNote (+ (Variables|Default|GetIndexOfButtonNote) 1)))

(event EventBeginPlay
  ;[1 0 0] BeginPlay
  (bind _returnvalue (Actor|GetActorOfClass "/Game/Test/Blueprint/Pawn/P_Player.P_Player_C"))
  (Variables|Default|SetP_Player _returnvalue))

(fn ConstructionScript)
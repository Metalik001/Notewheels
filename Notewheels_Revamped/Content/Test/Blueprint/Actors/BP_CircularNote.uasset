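; Circular rhythm-game note actor that scores when pressed inside a narrow radius window, otherwise failing with a bad sound and combo reset.
; A press in the window adds points and combo; a mistimed press or BeginPlay's timeout delay fails the note.
; A Timeline is meant to drive the dynamic sprite material's radius, thickness and green/red hit color, but nothing runs it in this graph.
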(event Custom|FailedNote
  ;[1 0 0] Begin Play
  (Audio|PlaySound2D "/Game/Test/Sound_Effects/SC_BadNote2_Cue.SC_BadNote2_Cue" 1.0 1.0 0.0 0 0)
  (Class|BPIGameMode|ResetCombo(Message) (Game|GetGameMode))
  (Actor|DestroyActor))

(event EventBeginPlay
  ;[1 0 0] Begin Play
  (Utilities|FlowControl|Delay (Variables|Default|GetTime%20to%20reach%20the%20end))
  (Audio|PlaySound2D "/Game/Test/Sound_Effects/SC_BadNote2_Cue.SC_BadNote2_Cue" 1.0 1.0 0.0 0 0)
  (Class|BPIGameMode|ResetCombo(Message) (Game|GetGameMode))
  (Actor|DestroyActor))

(event EventButtonPressed
  (bind _returnvalue (Game|GetGameMode))
  ;[1 1 1] Press Space
  ;[1 1 1] If successful
  (if (and (< (* (/ (stale _mouvement) (Variables|Default|GetTime%20to%20reach%20the%20end)) 0.35) 0.33) (> (* (/ (stale _mouvement) (Variables|Default|GetTime%20to%20reach%20the%20end)) 0.35) 0.28))
    (Audio|PlaySound2D "/Game/Test/Sound_Effects/SC_GoodNote_Cue.SC_GoodNote_Cue" 1.0 1.0 0.0 0 0)
    (Class|BPIGameMode|AddScore(Message) _returnvalue (Variables|Default|GetPointsToScore))
    (Class|BPIGameMode|AddNotetoCombo(Message) _returnvalue)
    (Actor|DestroyActor)
    (else
      (CallFunction|FailedNote))))

(fn ConstructionScript
  ;[1 1 1] Création du matérial
  (bind _returnvalue (Rendering|Material|CreateDynamicMaterialInstance (Variables|Default|GetPaperSprite) 0 "/Game/Test/Material/M_CircularNoteSprite.M_CircularNoteSprite" "None" :!class /Script/Engine.PrimitiveComponent))
  (Variables|Default|SetM_CircularNote _returnvalue))

(fn GetIndex
  (return (Variables|Default|GetIndex)))
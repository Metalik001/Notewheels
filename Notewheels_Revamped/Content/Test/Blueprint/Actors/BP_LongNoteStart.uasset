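; BP_LongNoteStart is the start piece of a long note, apparently for a rhythm game, that destroys itself after TimeToReachTheEnd.
; An overlap on its Background component reports its Index and itself to the game mode through TouchedLongNoteMessage.
; Timelines for moving it toward Destination and pitching the Note component are present but never triggered, so this graph does not animate it.
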(event OnComponentBeginOverlap(Background)
  (params (OverlappedComponent :type Primitive%20Component%20Object%20Reference) (OtherActor :type Actor%20Object%20Reference) (OtherComp :type Primitive%20Component%20Object%20Reference) (OtherBodyIndex :type Integer) (bFromSweep :type Boolean) (SweepResult :type Hit%20Result%20Structure%20%28by%20ref%29))
  ;[1 1 1] Stops the mouvement and make it disapear if the player touches it
  (Class|BPIGameMode|TouchedLongNote(Message) (Game|GetGameMode) (Variables|Default|GetIndex) self))

(event EventBeginPlay
  ;[1 0 0] When it's arrived, gets deleted
  (Utilities|FlowControl|Delay (Variables|Default|GetTime%20to%20reach%20the%20end))
  (Actor|DestroyActor))

(fn ConstructionScript)
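; Circular rhythm-game note actor that must be hit as its ring reaches a narrow radius window, then mashed a set number of times.
; A timeline drives the radius and thickness of a dynamic sprite material.
; A timed hit reveals the countdown and restarts the ring in reverse with a confirmation time limit.
; Presses add score, the last grants bonus points and combo, while mistimed presses or timeouts reset the combo and destroy the note.
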(event Custom|FailedNote
  ;[1 0 0] Begin Play
  (Audio|PlaySound2D "/Game/Test/Sound_Effects/SC_BadNote2_Cue.SC_BadNote2_Cue" 1.0 1.0 0.0 0 0)
  (Class|BPIGameMode|ResetCombo(Message) (Game|GetGameMode))
  (Actor|DestroyActor))

(event Custom|MashEvent
  (bind _returnvalue (Game|GetGameMode))
  (if (<= (Variables|Default|GetTimesToMash) 1)
    ;[1 1 1] Confirmed note
    (Audio|PlaySound2D "/Game/Test/Sound_Effects/SC_GoodNote_Cue.SC_GoodNote_Cue" 1.0 1.0 0.0 0 0)
    (Class|BPIGameMode|AddScore(Message) _returnvalue (* (Variables|Default|GetPointsToScore) 5))
    (Class|BPIGameMode|AddNotetoCombo(Message) _returnvalue)
    (Actor|DestroyActor)
    (else
      ;[1 1 1] Mashing
      (bind _result (Math|Integer|DecrementInt (Variables|Default|GetTimesToMash))
        (:%20%20
          (Rendering|Components|TextRender|SetText (Variables|Default|GetAmountOfTimesToTypeText) (Utilities|Text|ToText(Integer) _result))
          (Audio|PlaySound2D "/Game/Test/Sound_Effects/SC_GoodNote_Cue.SC_GoodNote_Cue" 1.0 1.0 0.0 0 0)
          (Class|BPIGameMode|AddScore(Message) (Game|GetGameMode) (Variables|Default|GetPointsToScore)))))))

(event Custom|Return%20to%20point
  (bind _m_circularnote (Variables|Default|GetM_CircularNote))
  (bind _time_to_reach_the_end (Variables|Default|GetTime%20to%20reach%20the%20end))
  (Utilities|FlowControl|Sequence
    (:then_0
      (bind _mouvement (Timeline|Timeline SetNewTime)
        (:Update
          ;[1 1 1] Movement
          (Rendering|Material|SetScalarParameterValue _m_circularnote "Radius" (* (/ _mouvement _time_to_reach_the_end) (Variables|Default|GetRingDistanceFromCenter)) :!class /Script/Engine.MaterialInstanceDynamic)
          (Rendering|Material|SetScalarParameterValue _m_circularnote "LineThickness" (- (* (/ _mouvement _time_to_reach_the_end) (Variables|Default|GetRingDistanceFromCenter)) 0.015) :!class /Script/Engine.MaterialInstanceDynamic))
        (:Finished
          (CallFunction|FailedNote))))
    (:then_1
      (Timeline|Timeline Reverse))))

(event EventBeginPlay
  ;[1 0 0] Begin Play
  (Utilities|FlowControl|Delay (Variables|Default|GetTime%20to%20reach%20the%20end))
  (if (not (Variables|Default|GetMashMode))
    (Audio|PlaySound2D "/Game/Test/Sound_Effects/SC_BadNote2_Cue.SC_BadNote2_Cue" 1.0 1.0 0.0 0 0)
    (Class|BPIGameMode|ResetCombo(Message) (Game|GetGameMode))
    (Actor|DestroyActor)))

(event EventButtonPressed
  (bind _amountoftimestotypetext (Variables|Default|GetAmountOfTimesToTypeText))
  ;[1 1 1] Press Space
  ;[1 1 1] If successfully hit once
  (if (Variables|Default|GetMashMode)
    (CallFunction|MashEvent)
    (elif (and (< (* (/ (stale Custom|Return%20to%20point _mouvement) (Variables|Default|GetTime%20to%20reach%20the%20end)) (Variables|Default|GetRingDistanceFromCenter)) 0.34) (> (* (/ (stale Custom|Return%20to%20point _mouvement) (Variables|Default|GetTime%20to%20reach%20the%20end)) (Variables|Default|GetRingDistanceFromCenter)) 0.3))
      (Variables|Default|SetMashMode true)
      (Utilities|FlowControl|DoOnce false
        (:Completed
          (Variables|Default|SetTime%20To%20Reach%20The%20End (Variables|Default|GetTime%20To%20ConfirmNote))
          (Development|SetHiddeninGame _amountoftimestotypetext false false)
          (Rendering|Components|TextRender|SetText _amountoftimestotypetext (Utilities|Text|ToText(Integer) (Variables|Default|GetTimesToMash)))
          (Variables|Default|SetRingDistanceFromCenter 0.3)
          (CallFunction|ReturntoPoint)))
      (else
        (CallFunction|FailedNote)))))

(fn ConstructionScript
  ;[1 1 1] Création du matérial
  (bind _returnvalue (Rendering|Material|CreateDynamicMaterialInstance (Variables|Default|GetPaperSprite) 0 "/Game/Test/Material/M_CircularNoteSprite.M_CircularNoteSprite" "None" :!class /Script/Engine.PrimitiveComponent))
  (bind _output_get (Variables|Default|SetM_CircularNote _returnvalue))
  (Rendering|Material|SetVectorParameterValue _output_get "Color" "(R=0.326956,G=0.052440,B=0.000000,A=1.000000)" :!class /Script/Engine.MaterialInstanceDynamic))

(fn GetIndex
  (return (Variables|Default|GetIndex)))
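; Rhythm-game note actor that moves toward a destination on the Movement timeline, lerped over TimeToReachTheEnd.
; Overlapping its Background stops and hides it, plays the good sound, then after a short delay adds score and combo through the game mode and destroys it.
; Points triple when the music frame saved on ButtonPressed is recent within Tolerance.
; When travel time expires, it plays the bad sound, resets combo and self-destroys if untouched.
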(event OnComponentBeginOverlap(Background)
  (params (OverlappedComponent :type Primitive%20Component%20Object%20Reference) (OtherActor :type Actor%20Object%20Reference) (OtherComp :type Primitive%20Component%20Object%20Reference) (OtherBodyIndex :type Integer) (bFromSweep :type Boolean) (SweepResult :type Hit%20Result%20Structure%20%28by%20ref%29))
  ;[1 1 1] Stops the mouvement and make it disapear if the player touches it
  (CallFunction|StopMovement)
  (Variables|Default|SetTouched true)
  (Development|SetHiddeninGame (Variables|Default|GetDefaultSceneRoot) true true)
  (Audio|PlaySound2D "/Game/Test/Sound_Effects/SC_GoodNote_Cue.SC_GoodNote_Cue" 1.0 1.0 0.0 0 0)
  (Utilities|FlowControl|Delay 0.2)
  (bind _currenttime (Class|BPIGameMode|GetCurrentMusicTime(Message) (Game|GetGameMode)))
  (if (>= (Variables|Default|GetFrameClicked) (- (Utilities|Struct|BreakFrameNumber (.Frame (Utilities|TimeManagement|BreakQualifiedFrameTime _currenttime))) (Variables|Default|GetTolerance)))
    (Variables|Default|SetPointsToScore (* (Variables|Default|GetPointsToScore) 3)))
  (Class|BPIGameMode|AddScore(Message) (Game|GetGameMode) (Variables|Default|GetPointsToScore))
  (Class|BPIGameMode|AddNotetoCombo(Message) (Game|GetGameMode))
  (Actor|DestroyActor))

(event Custom|StopMovement
  (bind _time_to_reach_the_end (Variables|Default|GetTime%20to%20reach%20the%20end))
  ;[1 1 1] Move Towards the end
  (bind _mouvement (Timeline|Movement Stop)
    (:Update
      (Transformation|SetRelativeLocation (Variables|Default|GetDefaultSceneRoot) (+ (Math|Vector|Lerp(Vector) "0, 0, 0" (Variables|Default|GetDestination) (/ _mouvement _time_to_reach_the_end)) "0.000000,0.000000,5.000000") false false))))

(event EventBeginPlay
  ;[1 0 0] When it's arrived, gets deleted
  (Utilities|FlowControl|Delay (Variables|Default|GetTime%20to%20reach%20the%20end))
  (Audio|PlaySound2D "/Game/Test/Sound_Effects/SC_BadNote_Cue.SC_BadNote_Cue" 1.0 1.0 0.0 0 0)
  (Class|BPIGameMode|ResetCombo(Message) (Game|GetGameMode))
  (if (not (Variables|Default|GetTouched))
    (Actor|DestroyActor)))

(event EventButtonPressed
  ;[1 1 1] Button effect
  (bind _currenttime (Class|BPIGameMode|GetCurrentMusicTime(Message) (Game|GetGameMode)))
  (Variables|Default|SetFrameClicked (Utilities|Struct|BreakFrameNumber (.Frame (Utilities|TimeManagement|BreakQualifiedFrameTime _currenttime)))))

(fn ConstructionScript)

(fn GetIndex
  (return (Variables|Default|GetIndex)))
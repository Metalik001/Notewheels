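; BP_SpikyRoll procedurally builds a spiky roll prop from static meshes laid along a spline.
; The construction script places a head mesh at spline point 1, then repeats body meshes at Offset intervals along the spline length, following its rotation.
; A FlipFlop alternates a 45-degree roll offset between segments to stagger them.
; The event graph has no active logic.
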(event EventBeginPlay)

(event Collision|EventActorBeginOverlap
  (params (OtherActor :type Actor%20Object%20Reference)))

(event EventTick
  (params (DeltaSeconds :type Float%20%28single-precision%29)))

(fn ConstructionScript
  (bind _offset (Variables|Default|Getoffset))
  (bind _spline (Variables|Default|GetSpline))
  ;[1 1 1] Tête
  (AddComponent|AddStaticMeshComponent false (Math|Transform|MakeTransform (.Position (Utilities|Struct|BreakSplinePoint (Spline|GetSplinePointAt (Variables|Default|GetSpline) 1 "Local"))) "-90.000000,0.000000,0.000000"))
  ;[1 1 1] Corps
  (for _index (range 0 (Math|Float|Floor (/ (Spline|GetSplineLength (Variables|Default|GetSpline)) _offset)))
    (Utilities|FlowControl|FlipFlop
      (:A
        (Variables|Default|SetRotoffset 0.0))
      (:B
        (Variables|Default|SetRotoffset 45.0)))
    (AddComponent|AddStaticMeshComponent false (Math|Transform|MakeTransform (Spline|GetLocationatDistanceAlongSpline _spline (* _index _offset) "Local") (Math|Rotator|MakeRotator (- (.Roll (Math|Rotator|BreakRotator (Spline|GetRotationatDistanceAlongSpline _spline (* _index _offset) "Local"))) (Variables|Default|GetRotoffset)) (.Pitch (Math|Rotator|BreakRotator (Spline|GetRotationatDistanceAlongSpline _spline (* _index _offset) "Local"))) (.Yaw (Math|Rotator|BreakRotator (Spline|GetRotationatDistanceAlongSpline _spline (* _index _offset) "Local"))))))))